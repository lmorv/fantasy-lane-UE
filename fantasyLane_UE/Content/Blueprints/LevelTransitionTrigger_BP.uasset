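; Level transition trigger that loads a named level when the player character overlaps its box, gated behind an optional voice-over.
; On BeginPlay it plays the voice-over track and delays for its duration, then toggles the sphere's visibility and opens a Gate.
; Without a valid track it toggles both the sphere and the Gate immediately.
; Player overlaps enter the Gate, which calls the level load only while open.
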(event `self.ReceiveBeginPlay`
  ;[1 1 1] VoiceOverDelay
  (`AudioComponent.SetSound` (`self.VO_Component`) (`self.VO_Track`))
  (`/Engine/EditorBlueprintResources/StandardMacros.IsValid` (`self.VO_Track`)
    (:`Is Valid`
      (`AudioComponent.Play` (`self.VO_Component`) 0.0)
      (`KismetSystemLibrary.Delay` (`SoundBase.Duration` (`self.VO_Track`)))
      (`SceneComponent.ToggleVisibility` (`self.Sphere`) false)
      (goto _label :!via `Open`))
    (:`Is Not Valid`
      (`SceneComponent.ToggleVisibility` (`self.Sphere`) false)
      (goto _label :!via `Toggle`))))

(event `self.Box.OnComponentBeginOverlap`
  (params (OverlappedComponent :type "PrimitiveComponent Object Reference") (OtherActor :type "Actor Object Reference") (OtherComp :type "PrimitiveComponent Object Reference") (OtherBodyIndex :type Integer) (bFromSweep :type Boolean) (SweepResult :type "HitResult Structure (by ref)"))
  (if (== OtherActor (`GameplayStatics.GetPlayerCharacter` 0))
    (`/Engine/EditorBlueprintResources/StandardMacros.Gate` true :!label _label
      (:`Exit`
        (`GameplayStatics.OpenLevel` (`self.Level Name`))))))

(fn `UserConstructionScript`)